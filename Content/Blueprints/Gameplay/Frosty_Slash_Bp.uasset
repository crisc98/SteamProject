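; Frosty's slash attack actor, which damages living enemies it overlaps on the server, once each, and multicasts ring hit particles.
; Unprimed enemies take base damage, scaled by Frosty's rage multiplier in rage mode; a non-rage hit also sets a short lifespan.
; Primed enemies trigger a Pop: a multicast lightning effect plus a server-side sphere trace that damages and unprimes nearby AI.
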(event `self.ReceiveBeginPlay`
  (`KismetSystemLibrary.PrintString` "Slash Created"))

(event `MulticastEnemyHitParticles`
  (params (AttachToComponent :type "SceneComponent Object Reference"))
  (`GameplayStatics.SpawnEmitterAttached` "/Game/Particles/RingFX.RingFX" AttachToComponent "None" (0.0 0.0 0.0) (struct) (0.8 0.8 0.8)))

(event `self.Box.OnComponentBeginOverlap`
  (params (OverlappedComponent :type "PrimitiveComponent Object Reference") (OtherActor :type "Actor Object Reference") (OtherComp :type "PrimitiveComponent Object Reference") (OtherBodyIndex :type Integer) (bFromSweep :type Boolean) (SweepResult :type "HitResult Structure (by ref)"))
  (bind _returnvalue (`self.GetOwner`))
  (bind _hitactors (`self.HitActors`))
  (bind _asfrosty (cast `/Game/Blueprints/Characters/Frosty` (`self.GetOwner`) :!pure true))
  (`/Engine/EditorBlueprintResources/ActorMacros.Switch Has Authority`
    (:`Authority`
      (if (`self.ActorHasTag` OtherActor "Enemy")
        (bind _asai_base (cast `/Game/Blueprints/Characters/AI_Base` OtherActor))
        (if (not (`/Game/Blueprints/Characters/AI_Base.IsDead` _asai_base))
          (set `self.HitEnemy` _asai_base)
          (if (not (`KismetArrayLibrary.Array_Contains` _hitactors (`self.HitEnemy`)))
            (`KismetArrayLibrary.Array_Add` _hitactors (`self.HitEnemy`))
            (`self.MulticastEnemyHitParticles` OtherComp)
            (if (`/Game/Blueprints/Characters/AI_Base.IsPrimed` (`self.HitEnemy`))
              (`self.Pop` (`self.HitEnemy`) (`self.GetOwner`) 100 "/Game/Particles/Lightning_Pop_FX.Lightning_Pop_FX")
              (elif (`/Game/Blueprints/Characters/Frosty.IsInRageMode` _asfrosty)
                (`/Game/Blueprints/Characters/AI_Base.TakeHit` (`self.HitEnemy`) _returnvalue (* (`self.Damage`) (`/Game/Blueprints/Characters/Frosty.RageMultiplier` _asfrosty)))
                (else
                  (`/Game/Blueprints/Characters/AI_Base.TakeHit` (`self.HitEnemy`) _returnvalue (`self.Damage`))
                  (`self.SetLifeSpan` 1.0))))))))))

(event `Pop`
  (params (Target :type "/Game/Blueprints/Characters/AI_Base Object Reference") (Instigator :type "Actor Object Reference") (Damage :type Integer) (EmitterTemplate :type "ParticleSystem Object Reference"))
  (bind (_returnvalue_roll _returnvalue_pitch _returnvalue_yaw) (`KismetMathLibrary.BreakRotator` (`KismetMathLibrary.RandomRotator` false)))
  (bind (_returnvalue_x _returnvalue_y _returnvalue_z) (`KismetMathLibrary.BreakVector` (`self.K2_GetActorLocation` Target)))
  ;[1 1 1] Pop Logic
  (`self.Multicast Spawn Pop FX` (`KismetMathLibrary.MakeVector` _returnvalue_x _returnvalue_y (- _returnvalue_z (`CapsuleComponent.CapsuleHalfHeight` (`Character.CapsuleComponent` Target)))) (`KismetMathLibrary.MakeRotator` 0.0 0.0 _returnvalue_yaw) EmitterTemplate))

(event `Multicast Spawn Pop FX`
  (params (Location :type "Vector Structure") (Rotation :type "Rotator Structure") (EmitterTemplate :type "ParticleSystem Object Reference"))
  ;[1 1 1] Pop Logic
  (`GameplayStatics.SpawnEmitterAtLocation` EmitterTemplate Location Rotation)
  (`/Engine/EditorBlueprintResources/ActorMacros.Switch Has Authority`
    (:`Authority`
      (`KismetArrayLibrary.Array_Clear` (`self.HitActors`))
      (bind _returnvalue (`self.K2_GetActorLocation` (stale `Pop` Target)))
      (bind _outhits (`KismetSystemLibrary.SphereTraceMulti` _returnvalue _returnvalue 500.0 "TraceTypeQuery1"))
      (for _array_element _outhits
        (bind _asai_base (cast `/Game/Blueprints/Characters/AI_Base` (`.HitActor` (`GameplayStatics.BreakHitResult` _array_element))))
        (if (not (`KismetArrayLibrary.Array_Contains` (`self.HitActors`) _asai_base))
          (`/Game/Blueprints/Characters/AI_Base.TakeHit` _asai_base (stale `Pop` Instigator) (stale `Pop` Damage))
          (`KismetArrayLibrary.Array_Add` (`self.HitActors`) _asai_base)
          (`/Game/Blueprints/Characters/AI_Base.UnPrime` _asai_base))))))

(fn `UserConstructionScript`)