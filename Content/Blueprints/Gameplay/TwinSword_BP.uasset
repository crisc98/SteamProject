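; Twin sword weapon actor for the Frosty character that detects basic-attack hits on walls and AI_Base enemies.
; Hits come from a blade collider overlap or a Base-to-Tip socket trace in ClientEventTick, which nothing here calls.
; Each enemy is hit once per attack, taking damage, granting rage and healing Frosty during rage mode.
; Multicast events re-trace the blade to place spark and splatter effects.
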(event `Server Wall Particles`
  (`self.MulticastWallParticles`))

(event `MulticastWallParticles`
  (bind _sword (`self.Sword`))
  (bind (_outhit _returnvalue) (`KismetSystemLibrary.LineTraceSingle` :`Start` (`SceneComponent.GetSocketLocation` _sword "Base") :`End` (`SceneComponent.GetSocketLocation` _sword "Tip") :`TraceChannel` "TraceTypeQuery1" :`DrawTime` 0.5))
  (if _returnvalue
    (`GameplayStatics.SpawnEmitterAtLocation` "/Game/Particles/Wall_Hit_Sparks.Wall_Hit_Sparks" (`.Location` (`GameplayStatics.BreakHitResult` _outhit)) (struct) (`KismetMathLibrary.Conv_DoubleToVector` (`KismetMathLibrary.RandomFloatInRange` 0.5)))))

(event `SetParticleTrail`
  (params (Trail :type "ParticleSystem Object Reference"))
  ;[1 1 1] Set Weapon Particle Trail
  (`ParticleSystemComponent.SetTemplate` (`self.Trail`) Trail))

(event `self.ReceiveBeginPlay`
  (bind _asfrosty (cast `/Game/Blueprints/Characters/Frosty` (`self.GetOwner`)))
  (set `self.CharacterRef` _asfrosty))

(event `Server Hit Particles`
  (`self.MulticastHitParticles`))

(event `ClientEventTick`
  (bind _characterref (`self.CharacterRef`))
  (bind _characterref_2 (`self.CharacterRef`))
  (bind _sword (`self.Sword`))
  (bind _enemieshitinattack (`/Game/Blueprints/Characters/Frosty.EnemiesHitInAttack` (`self.CharacterRef`)))
  (bind _activeweapondamage (`/Game/Blueprints/Characters/Frosty.ActiveWeaponDamage` _characterref_2))
  (bind _asfrosty (cast `/Game/Blueprints/Characters/Frosty` (`self.GetOwner`)))
  (set `self.CharacterRef` _asfrosty)
  (if (and (`/Game/Blueprints/Characters/Frosty.IsBasicAttacking` _asfrosty) (`/Game/Blueprints/Characters/Frosty.WeaponDamageEnabled` _asfrosty))
    (bind (_outhit _returnvalue) (`KismetSystemLibrary.LineTraceSingle` :`Start` (`SceneComponent.GetSocketLocation` _sword "Base") :`End` (`SceneComponent.GetSocketLocation` _sword "Tip") :`TraceChannel` "TraceTypeQuery1" :`DrawTime` 0.5))
    (if _returnvalue
      (bind (_bblockinghit _binitialoverlap _time _distance _location _impactpoint _normal _impactnormal _physmat _hitactor _hitcomponent) (`GameplayStatics.BreakHitResult` _outhit))
      (switch `ECollisionChannel` (`PrimitiveComponent.GetCollisionObjectType` _hitcomponent)
        (:`ECC_WorldStatic`
          (`self.MulticastWallParticles`))
        (:`ECC_Pawn`
          (bind _asai_base (cast `/Game/Blueprints/Characters/AI_Base` _hitactor))
          (set `self.HitEnemy` _asai_base)
          (if (not (`KismetArrayLibrary.Array_Contains` _enemieshitinattack _asai_base))
            (`KismetArrayLibrary.Array_Add` _enemieshitinattack _asai_base)
            (`/Game/Blueprints/Characters/Frosty.GainRage` _characterref 5)
            (if (`/Game/Blueprints/Characters/Frosty.IsInRageMode` _characterref)
              (`/Game/Blueprints/Characters/0_Base.Heal` _characterref (`KismetMathLibrary.FTrunc` (* _activeweapondamage (`/Game/Blueprints/Characters/Frosty.RageLifestealMultiplier` _characterref_2)))))
            (`/Game/Blueprints/Characters/AI_Base.TakeHit` _asai_base _characterref_2 _activeweapondamage)
            (`self.MulticastHitParticles`)
            (`/Game/Blueprints/Characters/AI_Base.ClientDamageWidget` (`self.HitEnemy`) _activeweapondamage)))))))

(event `self.ReceiveTick`
  (params (DeltaSeconds :type "Float (single-precision)")))

(event `MulticastHitParticles`
  (bind _sword (`self.Sword`))
  (bind (_outhit _returnvalue) (`KismetSystemLibrary.LineTraceSingle` :`Start` (`SceneComponent.GetSocketLocation` _sword "Base") :`End` (`SceneComponent.GetSocketLocation` _sword "Tip") :`TraceChannel` "TraceTypeQuery1" :`DrawTime` 0.5))
  (if _returnvalue
    (`GameplayStatics.SpawnEmitterAtLocation` "/Game/Particles/Splatters.Splatters" (`.Location` (`GameplayStatics.BreakHitResult` _outhit)))))

(event `self.BladeCollider.OnComponentBeginOverlap`
  (params (OverlappedComponent :type "PrimitiveComponent Object Reference") (OtherActor :type "Actor Object Reference") (OtherComp :type "PrimitiveComponent Object Reference") (OtherBodyIndex :type Integer) (bFromSweep :type Boolean) (SweepResult :type "HitResult Structure (by ref)"))
  (bind _characterref (`self.CharacterRef`))
  (bind _characterref_2 (`self.CharacterRef`))
  (bind _characterref_3 (`self.CharacterRef`))
  ;[1 1 1] Hit logic using overlap
  (if (`/Game/Blueprints/Characters/Frosty.IsBasicAttacking` (`self.CharacterRef`))
    (switch `ECollisionChannel` (`PrimitiveComponent.GetCollisionObjectType` OtherComp)
      (:`ECC_WorldStatic`
        (`self.Server Wall Particles`))
      (:`ECC_Pawn`
        (bind _asai_base (cast `/Game/Blueprints/Characters/AI_Base` OtherActor))
        (set `self.HitEnemy` _asai_base)
        (if (not (`KismetArrayLibrary.Array_Contains` (`/Game/Blueprints/Characters/Frosty.EnemiesHitInAttack` (`self.CharacterRef`)) _asai_base))
          (`KismetArrayLibrary.Array_Add` (`/Game/Blueprints/Characters/Frosty.EnemiesHitInAttack` (`self.CharacterRef`)) (`self.HitEnemy`))
          (`/Game/Blueprints/Characters/Frosty.GainRage` _characterref 5)
          (if (`/Game/Blueprints/Characters/Frosty.IsInRageMode` _characterref)
            (`/Game/Blueprints/Characters/0_Base.Heal` (`self.CharacterRef`) (`KismetMathLibrary.FTrunc` (* (`/Game/Blueprints/Characters/Frosty.ActiveWeaponDamage` _characterref_3) (`/Game/Blueprints/Characters/Frosty.RageLifestealMultiplier` _characterref_3)))))
          (`/Game/Blueprints/Characters/AI_Base.TakeHit` (`self.HitEnemy`) _characterref_2 (`/Game/Blueprints/Characters/Frosty.ActiveWeaponDamage` _characterref_2))
          (if (not (`/Game/Blueprints/Characters/AI_Base.IsDead` (`self.HitEnemy`)))
            (`self.Server Hit Particles`)))))))

(fn `UserConstructionScript`)