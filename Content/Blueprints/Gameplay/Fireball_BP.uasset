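; Fireball projectile owned by Tusk that explodes when its capsule overlaps an actor tagged Walkable or Enemy.
; The explosion spawns a scaled-down meteor emitter and runs a multi-sphere trace around the capsule.
; Each unique AI_Base found takes fireball damage once, tracked through a HitActors list, and gets primed with a timed fire effect on the hit bone.
; A successful hit also sets a short lifespan on the fireball.
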(event `self.ReceiveBeginPlay`)

(event `self.Capsule.OnComponentBeginOverlap`
  (params (OverlappedComponent :type "PrimitiveComponent Object Reference") (OtherActor :type "Actor Object Reference") (OtherComp :type "PrimitiveComponent Object Reference") (OtherBodyIndex :type Integer) (bFromSweep :type Boolean) (SweepResult :type "HitResult Structure (by ref)"))
  (if (or (`self.ActorHasTag` OtherActor "Walkable") (`self.ActorHasTag` OtherActor "Enemy"))
    (`GameplayStatics.SpawnEmitterAtLocation` "/Game/Particles/Par_Meteora_Explode_01.Par_Meteora_Explode_01" (`SceneComponent.K2_GetComponentLocation` (`self.Capsule`)) (struct) (0.4 0.4 0.4))
    (`self.DamageAllActorsInRadius`)))

(event `DamageAllActorsInRadius`
  (bind _returnvalue (`SceneComponent.K2_GetComponentLocation` (`self.Capsule`)))
  (cast `/Game/Blueprints/Characters/Tusk` (`self.GetOwner`))
  (`KismetArrayLibrary.Array_Clear` (`self.HitActors`))
  (bind _outhits (`KismetSystemLibrary.SphereTraceMulti` _returnvalue _returnvalue 275.0 "TraceTypeQuery1"))
  (for _array_element _outhits
    (bind (_bblockinghit _binitialoverlap _time _distance _location _impactpoint _normal _impactnormal _physmat _hitactor _hitcomponent _hitbonename) (`GameplayStatics.BreakHitResult` _array_element))
    (bind _asai_base (cast `/Game/Blueprints/Characters/AI_Base` _hitactor))
    (if (not (`KismetArrayLibrary.Array_Contains` (`self.HitActors`) _asai_base))
      (`/Game/Blueprints/Characters/AI_Base.TakeHit` _asai_base (`self.GetOwner`) (`KismetMathLibrary.FTrunc` (`self.FireballDamage`)))
      (`KismetArrayLibrary.Array_Add` (`self.HitActors`) _asai_base)
      (`/Game/Blueprints/Characters/AI_Base.Prime` _asai_base "/Game/Particles/Fire_Prime_FX.Fire_Prime_FX" _hitcomponent _hitbonename 5.0)
      (`self.SetLifeSpan` 0.3))))

(fn `UserConstructionScript`)