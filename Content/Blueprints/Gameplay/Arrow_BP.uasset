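; Arrow actor that damages characters derived from 0_Base when its head collider strikes them.
; Only overlaps with the character's capsule count, and a HitActors list limits each arrow to one hit per character.
; A hit applies ArrowDamage and plays a world camera shake centred on the victim's follow camera, with a tiny radius that confines it to that view.
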(event `self.HeadCollider.OnComponentBeginOverlap`
  (params (OverlappedComponent :type "PrimitiveComponent Object Reference") (OtherActor :type "Actor Object Reference") (OtherComp :type "PrimitiveComponent Object Reference") (OtherBodyIndex :type Integer) (bFromSweep :type Boolean) (SweepResult :type "HitResult Structure (by ref)"))
  (bind _as0_base (cast `/Game/Blueprints/Characters/0_Base` OtherActor))
  (if (== (`Character.CapsuleComponent` _as0_base) OtherComp)
    (if (not (`KismetArrayLibrary.Array_Contains` (`self.HitActors`) _as0_base))
      (`GameplayStatics.PlayWorldCameraShake` "/Game/UI/HitCameraShake.HitCameraShake_C" (`SceneComponent.K2_GetComponentLocation` (`/Game/Blueprints/Characters/0_Base.FollowCamera` _as0_base)) 0.0 0.5 0.0)
      (`GameplayStatics.ApplyDamage` _as0_base (`self.ArrowDamage`) null self)
      (`KismetArrayLibrary.Array_Add` (`self.HitActors`) _as0_base))))

(fn `UserConstructionScript`)