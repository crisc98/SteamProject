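; TuskBA_BP is the hit actor for Tusk's basic attack, damaging enemies its capsule overlaps.
; Each AI_Base tagged Enemy gets one hit effect, tracked through HitActors.
; If that enemy is not primed, the server applies damage, grants mana to the owning Tusk and sets a very short lifespan.
; Overlapping Walkable actors without the Enemy tag spawns the effect and destroys the actor immediately.
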(event `self.Capsule.OnComponentBeginOverlap`
  (params (OverlappedComponent :type "PrimitiveComponent Object Reference") (OtherActor :type "Actor Object Reference") (OtherComp :type "PrimitiveComponent Object Reference") (OtherBodyIndex :type Integer) (bFromSweep :type Boolean) (SweepResult :type "HitResult Structure (by ref)"))
  (bind _hitactors (`self.HitActors`))
  ;[1 1 1] Collison logic
  (if (`self.ActorHasTag` OtherActor "Enemy")
    (bind _asai_base (cast `/Game/Blueprints/Characters/AI/AI_Base` OtherActor))
    (if (not (`KismetArrayLibrary.Array_Contains` _hitactors _asai_base))
      (`KismetArrayLibrary.Array_Add` _hitactors _asai_base)
      (`GameplayStatics.SpawnEmitterAttached` "/Game/Particles/Tusk_Basic_Hit_FX.Tusk_Basic_Hit_FX" OtherComp "None" (0.0 0.0 0.0) (struct) (0.3 0.3 0.3))
      (if (not (`/Game/Blueprints/Characters/AI/AI_Base.IsPrimed` _asai_base))
        (`/Engine/EditorBlueprintResources/ActorMacros.Switch Has Authority`
          (:`Authority`
            (`/Game/Blueprints/Characters/AI/AI_Base.TakeHit` _asai_base (`self.GetOwner`) (`self.Damage`))
            (bind _astusk (cast `/Game/Blueprints/Characters/Tusk` (`self.GetOwner`)))
            (`/Game/Blueprints/Characters/Tusk.Gain Mana` _astusk 5.0)
            (`self.SetLifeSpan` 0.05)))))
    (elif (`self.ActorHasTag` OtherActor "Walkable")
      (`GameplayStatics.SpawnEmitterAtLocation` "/Game/Particles/Tusk_Basic_Hit_FX.Tusk_Basic_Hit_FX" (`self.K2_GetActorLocation`) (struct) (0.3 0.3 0.3))
      (`self.K2_DestroyActor`))))

(fn `UserConstructionScript`)