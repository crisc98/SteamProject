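; Tusk basic-attack hit actor that damages enemies and sets off area "pops" on primed ones.
; Wrapper overlap plays hit FX, then either pops a primed AI_Base or applies direct damage on authority, and sets a short lifespan.
; Pops multicast lightning FX, while authority sphere-traces to damage and unprime each unique enemy, granting Tusk mana per enemy.
; Overlapping non-enemy Walkable actors spawns hit FX and destroys the actor.
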(event `self.Wrapper.OnComponentBeginOverlap`
  (params (OverlappedComponent :type "PrimitiveComponent Object Reference") (OtherActor :type "Actor Object Reference") (OtherComp :type "PrimitiveComponent Object Reference") (OtherBodyIndex :type Integer) (bFromSweep :type Boolean) (SweepResult :type "HitResult Structure (by ref)"))
  (bind _returnvalue (`self.GetOwner`))
  (bind _hitactors (`self.HitActors`))
  (bind _hitenemyref (`self.HitEnemyRef`))
  ;[1 1 1] Collison logic
  (if (`self.ActorHasTag` OtherActor "Enemy")
    (bind _asai_base (cast `/Game/Blueprints/Characters/AI_Base` OtherActor))
    (set `self.HitEnemyRef` _asai_base)
    (`KismetArrayLibrary.Array_Clear` _hitactors)
    (if (not (`KismetArrayLibrary.Array_Contains` _hitactors _hitenemyref))
      (`KismetArrayLibrary.Array_Add` _hitactors (`self.HitEnemyRef`))
      (`GameplayStatics.SpawnEmitterAttached` "/Game/Particles/Tusk_BA_Hit_FX.Tusk_BA_Hit_FX" OtherComp "None" (0.0 0.0 0.0) (struct) (0.8 0.8 0.8))
      (if (`/Game/Blueprints/Characters/AI_Base.IsPrimed` _hitenemyref)
        (`self.Pop` (`self.HitEnemyRef`) _returnvalue (`self.PopDamage`) "/Game/Particles/Lightning_Pop_FX.Lightning_Pop_FX")
        (else
          (`/Engine/EditorBlueprintResources/ActorMacros.Switch Has Authority`
            (:`Authority`
              (`/Game/Blueprints/Characters/AI_Base.TakeHit` (`self.HitEnemyRef`) _returnvalue (`self.Damage`))))))
      (`self.SetLifeSpan` 1.0))
    (elif (`self.ActorHasTag` OtherActor "Walkable")
      (`GameplayStatics.SpawnEmitterAtLocation` "/Game/Particles/Tusk_BA_Hit_FX.Tusk_BA_Hit_FX" (`self.K2_GetActorLocation`) (struct) (0.8 0.8 0.8))
      (`self.K2_DestroyActor`))))

(event `Pop`
  (params (Target :type "/Game/Blueprints/Characters/AI_Base Object Reference") (Instigator :type "Actor Object Reference") (Damage :type Integer) (EmitterTemplate :type "ParticleSystem Object Reference"))
  (bind (_returnvalue_roll _returnvalue_pitch _returnvalue_yaw) (`KismetMathLibrary.BreakRotator` (`KismetMathLibrary.RandomRotator` false)))
  (bind (_returnvalue_x _returnvalue_y _returnvalue_z) (`KismetMathLibrary.BreakVector` (`self.K2_GetActorLocation` Target)))
  ;[1 1 1] Pop Logic
  (`self.Multicast Spawn Pop FX` (`KismetMathLibrary.MakeVector` _returnvalue_x _returnvalue_y (- _returnvalue_z (`CapsuleComponent.CapsuleHalfHeight` (`Character.CapsuleComponent` Target)))) (`KismetMathLibrary.MakeRotator` 0.0 0.0 _returnvalue_yaw) EmitterTemplate))

(event `Multicast Spawn Pop FX`
  (params (Location :type "Vector Structure") (Rotation :type "Rotator Structure") (EmitterTemplate :type "ParticleSystem Object Reference"))
  ;[1 1 1] Pop Logic
  (`GameplayStatics.SpawnEmitterAtLocation` EmitterTemplate Location Rotation)
  (`/Engine/EditorBlueprintResources/ActorMacros.Switch Has Authority`
    (:`Authority`
      (`KismetArrayLibrary.Array_Clear` (`self.HitActors`))
      (bind _returnvalue (`self.K2_GetActorLocation` (stale `Pop` Target)))
      (bind _outhits (`KismetSystemLibrary.SphereTraceMulti` _returnvalue _returnvalue 500.0 "TraceTypeQuery1"))
      (for _array_element _outhits
        (bind _asai_base (cast `/Game/Blueprints/Characters/AI_Base` (`.HitActor` (`GameplayStatics.BreakHitResult` _array_element))))
        (if (not (`KismetArrayLibrary.Array_Contains` (`self.HitActors`) _asai_base))
          (`/Game/Blueprints/Characters/AI_Base.TakeHit` _asai_base (stale `Pop` Instigator) (stale `Pop` Damage))
          (`KismetArrayLibrary.Array_Add` (`self.HitActors`) _asai_base)
          (`/Game/Blueprints/Characters/AI_Base.UnPrime` _asai_base)
          (bind _astusk (cast `/Game/Blueprints/Characters/Tusk` (`self.GetOwner`)))
          (`/Game/Blueprints/Characters/Tusk.Gain Mana` _astusk 50.0))))))

(fn `UserConstructionScript`)