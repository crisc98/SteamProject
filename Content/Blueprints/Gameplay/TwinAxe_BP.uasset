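; Twin axe melee weapon for the Frosty character that damages AI enemies and spawns impact effects.
; While mounted and the owner basic-attacks, blade overlaps hit each AI_Base once per attack, granting rage on living targets and lifesteal during rage mode.
; Wall and flesh impacts route through Server-to-Multicast events, which trace from Base to Tip sockets to place sparks or splatters.
; A separate event sets the particle trail template.
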(event `Server Wall Particles`
  (`self.MulticastWallParticles`))

(event `MulticastWallParticles`
  (bind _skeletalmesh (`self.SkeletalMesh`))
  (bind (_outhit _returnvalue) (`KismetSystemLibrary.LineTraceSingle` :`Start` (`SceneComponent.GetSocketLocation` _skeletalmesh "Base") :`End` (`SceneComponent.GetSocketLocation` _skeletalmesh "Tip") :`TraceChannel` "TraceTypeQuery1" :`DrawTime` 0.5))
  (if _returnvalue
    (`GameplayStatics.SpawnEmitterAtLocation` "/Game/Particles/Wall_Hit_Sparks.Wall_Hit_Sparks" (`.Location` (`GameplayStatics.BreakHitResult` _outhit)) (struct) (`KismetMathLibrary.Conv_DoubleToVector` (`KismetMathLibrary.RandomFloatInRange` 0.5)))))

(event `self.ReceiveBeginPlay`
  (bind _asfrosty (cast `/Game/Blueprints/Characters/Frosty` (`self.GetOwner`)))
  (set `self.CharacterRef` _asfrosty)
  (set `self.Mounted` true))

(event `SetParticleTrail`
  (params (Trail :type "ParticleSystem Object Reference"))
  ;[1 1 1] Set Weapon Particle Trail
  (`ParticleSystemComponent.SetTemplate` (`self.Trail`) Trail))

(event `Server Hit Particles`
  (`self.MulticastHitParticles`))

(event `MulticastHitParticles`
  (bind _skeletalmesh (`self.SkeletalMesh`))
  (bind (_outhit _returnvalue) (`KismetSystemLibrary.LineTraceSingle` :`Start` (`SceneComponent.GetSocketLocation` _skeletalmesh "Base") :`End` (`SceneComponent.GetSocketLocation` _skeletalmesh "Tip") :`TraceChannel` "TraceTypeQuery1" :`DrawTime` 0.5))
  (if _returnvalue
    (`GameplayStatics.SpawnEmitterAtLocation` "/Game/Particles/Splatters.Splatters" (`.Location` (`GameplayStatics.BreakHitResult` _outhit)))))

(event `self.BladeCollider.OnComponentBeginOverlap`
  (params (OverlappedComponent :type "PrimitiveComponent Object Reference") (OtherActor :type "Actor Object Reference") (OtherComp :type "PrimitiveComponent Object Reference") (OtherBodyIndex :type Integer) (bFromSweep :type Boolean) (SweepResult :type "HitResult Structure (by ref)"))
  ;[1 1 1] Hit logic using overlap
  (if (`self.Mounted`)
    (if (`/Game/Blueprints/Characters/Frosty.IsBasicAttacking` (`self.CharacterRef`))
      (switch `ECollisionChannel` (`PrimitiveComponent.GetCollisionObjectType` OtherComp)
        (:`ECC_WorldStatic`
          (`self.Server Wall Particles`))
        (:`ECC_Pawn`
          (bind _asai_base (cast `/Game/Blueprints/Characters/AI_Base` OtherActor))
          (set `self.HitEnemy` _asai_base)
          (if (not (`KismetArrayLibrary.Array_Contains` (`/Game/Blueprints/Characters/Frosty.EnemiesHitInAttack` (`self.CharacterRef`)) _asai_base))
            (`KismetArrayLibrary.Array_Add` (`/Game/Blueprints/Characters/Frosty.EnemiesHitInAttack` (`self.CharacterRef`)) (`self.HitEnemy`))
            (if (`/Game/Blueprints/Characters/Frosty.IsInRageMode` (`self.CharacterRef`))
              (`/Game/Blueprints/Characters/0_Base.Heal` (`self.CharacterRef`) (`KismetMathLibrary.FTrunc` (* (`/Game/Blueprints/Characters/Frosty.ActiveWeaponDamage` (`self.CharacterRef`)) (`/Game/Blueprints/Characters/Frosty.RageLifestealMultiplier` (`self.CharacterRef`))))))
            (`/Game/Blueprints/Characters/AI_Base.TakeHit` (`self.HitEnemy`) (`self.CharacterRef`) (`/Game/Blueprints/Characters/Frosty.ActiveWeaponDamage` (`self.CharacterRef`)))
            (if (not (`/Game/Blueprints/Characters/AI_Base.IsDead` (`self.HitEnemy`)))
              (`self.Server Hit Particles`)
              (`/Game/Blueprints/Characters/Frosty.GainRage` (`self.CharacterRef`) 5))))))))

(fn `UserConstructionScript`)