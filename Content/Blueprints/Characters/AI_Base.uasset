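; AI_Base is the enemy AI character with replicated health, a camera-facing health bar, death cleanup and angle-based hit reactions.
; Damage lowers CurrentHP on authority and triggers death at zero, while OnRep updates the bar.
; Attack, called with a behavior tree task, plays a random twin-sword montage and reports success or failure back to it.
; While attacking, Tick traces along the right arm, damaging each player once per swing.
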(event `DebugEventTick`
  (`KismetSystemLibrary.PrintString` (`KismetStringLibrary.Conv_DoubleToString` (`KismetMathLibrary.VSize` (`self.GetVelocity`))) true true (struct :`R` 0.771568 :`B` 1.0 :`A` 1.0) 0.0)
  (`KismetSystemLibrary.PrintString` (`KismetStringLibrary.Conv_BoolToString` (`self.IsHit`)) true true (struct :`R` 0.771568 :`B` 1.0 :`A` 1.0) 0.0))

(event `self.ReceiveTick`
  (params (DeltaSeconds :type "Float (single-precision)"))
  (`self.RotateHealthBarToPlayer`)
  (`self.CheckForArmHit`)
  (`self.DebugEventTick`))

(event `self.ReceiveBeginPlay`
  (`KismetSystemLibrary.PrintString` "AI Spawned")
  (bind _asenemy_health_wb (cast `/Game/UI/AllLevels/EnemyHealthWB` (`WidgetComponent.GetUserWidgetObject` (`self.HealthBar`))))
  (bind _output_get (set `self.HeathBarWB` _asenemy_health_wb))
  (set `/Game/UI/AllLevels/EnemyHealthWB.Health` (`self.CurrentHP`) _output_get)
  (set `/Game/UI/AllLevels/EnemyHealthWB.MaxHeath` (`self.MaxHP`) _output_get)
  (`/Game/UI/AllLevels/EnemyHealthWB.UpdateHealth` (`self.HeathBarWB`) (`KismetMathLibrary.Conv_IntToDouble` (`self.CurrentHP`))))

(event `self.ReceiveAnyDamage`
  (params (Damage :type "Float (single-precision)") (DamageType :type "DamageType Object Reference") (InstigatedBy :type "Controller Object Reference") (DamageCauser :type "Actor Object Reference"))
  ;[1 1 1] Take Damage Logic
  (`self.OnTakeDamage` (`KismetMathLibrary.FTrunc` Damage)))

(event `HandleDeath`
  (bind _capsulecomponent (`self.CapsuleComponent`))
  ;[1 1 1] Death Handler
  (`SceneComponent.SetVisibility` (`self.HealthBar`) false false)
  (set `self.IsDead` true)
  (`PrimitiveComponent.SetCollisionResponseToChannel` _capsulecomponent "ECC_Visibility" "ECR_Ignore")
  (`PrimitiveComponent.SetCollisionResponseToChannel` (`self.Mesh`) "ECC_Visibility" "ECR_Ignore")
  (`PrimitiveComponent.SetCollisionResponseToChannel` _capsulecomponent "ECC_Pawn" "ECR_Ignore")
  (`PrimitiveComponent.SetCollisionResponseToChannel` (`self.Mesh`) "ECC_Pawn" "ECR_Ignore")
  (`KismetSystemLibrary.Delay` 5.0)
  (`self.K2_DestroyActor`))

(event `CheckDead`
  ;[1 1 1] Check if character is dead
  (if (<= (`self.CurrentHP`) 0)
    (set `self.IsDead` true)
    (`self.HandleDeath`)))

(event `Heal`
  (params (HealHP :type Integer))
  ;[1 1 1] Heal for some amount of HP
  (bind _output_get (set `self.CurrentHP` (`KismetMathLibrary.Clamp` (+ HealHP (`self.CurrentHP`)) 0 (`self.MaxHP`))))
  (`/Game/UI/AllLevels/EnemyHealthWB.UpdateHealth` (`self.HeathBarWB`) (`KismetMathLibrary.Conv_IntToDouble` _output_get)))

(event `SetIsHit`
  (set `self.IsHit` true))

(event `ProcessHitReact`
  (params (Target :type "Actor Object Reference"))
  (bind _returnvalue_x (`KismetMathLibrary.BreakVector` (`self.K2_GetActorLocation`)))
  (bind _returnvalue_x_2 (`KismetMathLibrary.BreakVector` (`self.K2_GetActorLocation` Target)))
  (bind _returnvalue (`KismetMathLibrary.DegAcos` (`KismetMathLibrary.Dot_VectorVector` (`KismetMathLibrary.Normal` (`SceneComponent.GetForwardVector` (`self.Mesh`))) (`KismetMathLibrary.Normal` (`self.GetActorForwardVector` Target)))))
  ;[1 1 1] Hit Reaction logic
  (`self.MulticastStopMontage`)
  (if (< _returnvalue_x _returnvalue_x_2)
    (bind _output_get (set `self.HitAngle` (* _returnvalue -1.0)))
    (`KismetSystemLibrary.PrintString` (`KismetStringLibrary.Conv_DoubleToString` _output_get) true true (struct :`R` 1.0 :`G` 0.225598 :`A` 1.0))
    (else
      (bind _output_get_2 (set `self.HitAngle` _returnvalue))
      (`KismetSystemLibrary.PrintString` (`KismetStringLibrary.Conv_DoubleToString` _output_get_2) true true (struct :`R` 1.0 :`G` 0.225598 :`A` 1.0))))
  (`self.SetIsHit`))

(event `TakeHit`
  (params (Instigator :type "Character Object Reference") (Damage :type Integer))
  ;[1 1 1] Hit Reaction logic
  (`GameplayStatics.ApplyDamage` self (`KismetMathLibrary.Conv_IntToDouble` Damage))
  (`self.ProcessHitReact` Instigator))

(event `MulticastStopMontage`
  ;[1 1 1] Hit Reaction logic
  (`self.StopAnimMontage` null))

(event `MulticastResetHit`
  (set `self.IsHit` false))

(event `ResetHit`
  (`/Engine/EditorBlueprintResources/ActorMacros.Switch Has Authority`
    (:`Authority`
      (`self.MulticastResetHit`))
    (:`Remote`
      (`self.ClientResetHit`))))

(event `ClientResetHit`
  (`self.MulticastResetHit`))

(event `CheckForArmHit`
  (bind _mesh (`self.Mesh`))
  ;[1 1 1] Attack raycast logic
  (if (`self.IsAttacking`)
    (bind (_outhit _returnvalue) (`KismetSystemLibrary.LineTraceSingle` :`Start` (`SceneComponent.GetSocketLocation` _mesh "upperarm_r") :`End` (`SceneComponent.GetSocketLocation` _mesh "hand_rSocket") :`TraceChannel` "TraceTypeQuery1" :`DrawTime` 0.5))
    (if _returnvalue
      (bind _as0_base (cast `/Game/Blueprints/Characters/0_Base` (`.HitActor` (`GameplayStatics.BreakHitResult` _outhit))))
      (if (not (`KismetArrayLibrary.Array_Contains` (`self.HitActors`) _as0_base))
        (`GameplayStatics.PlayWorldCameraShake` "/Game/UI/HitCameraShake.HitCameraShake_C" (`SceneComponent.K2_GetComponentLocation` (`/Game/Blueprints/Characters/0_Base.FollowCamera` _as0_base)) 0.0 0.5)
        (`GameplayStatics.ApplyDamage` _as0_base (`self.BaseDamage`) null self)
        (`KismetArrayLibrary.Array_Add` (`self.HitActors`) _as0_base)))))

(event `Attack`
  (params (CallingTask :type "BTTask_BlueprintBase Object Reference"))
  ;[1 1 1] Attack logic
  (if (and (not (`NavMovementComponent.IsFalling` (`self.GetMovementComponent`))) (not (`self.IsReactingToHit`)) (not (`self.IsDead`)))
    (set `self.JumpEnabled` false)
    (set `self.IsAttacking` true)
    (`KismetArrayLibrary.Array_Clear` (`self.HitActors`))
    (`|PlayMontage` (`self.Mesh`) (select `int` (`KismetMathLibrary.RandomIntegerInRange` 0 7) :`0` "/Game/InfinityBladeWarriors/Animations/TwinSword_Attack01_Montage.TwinSword_Attack01_Montage" :`1` "/Game/InfinityBladeWarriors/Animations/TwinSword_Attack02_Montage.TwinSword_Attack02_Montage" :`2` "/Game/InfinityBladeWarriors/Animations/TwinSword_Attack03_Montage.TwinSword_Attack03_Montage" :`3` "/Game/InfinityBladeWarriors/Animations/TwinSword_Attack04_Montage.TwinSword_Attack04_Montage" :`4` "/Game/InfinityBladeWarriors/Animations/TwinSword_Attack05_Montage.TwinSword_Attack05_Montage" :`5` "/Game/InfinityBladeWarriors/Animations/TwinSword_Attack05_Montage.TwinSword_Attack05_Montage" :`6` "/Game/InfinityBladeWarriors/Animations/TwinSword_Attack06_Montage.TwinSword_Attack06_Montage" :`7` "/Game/InfinityBladeWarriors/Animations/TwinSword_Attack07_Montage.TwinSword_Attack07_Montage" :!type "AnimMontage Object Reference")
      (:`OnCompleted`
        (set `self.JumpEnabled` true)
        (set `self.IsAttacking` false)
        (`self.ResolveAttackCallback` CallingTask))
      (:`OnInterrupted`
        (set `self.JumpEnabled` true)
        (set `self.IsAttacking` false)
        (`self.RejectAttackCallback` CallingTask)))
    (else
      (`self.RejectAttackCallback` CallingTask))))

(event `ResolveAttackCallback`
  (params (CallingTask :type "Object Object Reference"))
  ;[1 1 1] Attack logic
  (cast `/Game/AI/Tasks/AttackPawn_BTTask` CallingTask)
  (`BTTask_BlueprintBase.FinishExecute` (stale `Attack` CallingTask) true))

(event `RejectAttackCallback`
  (params (CallingTask :type "BTTask_BlueprintBase Object Reference"))
  ;[1 1 1] Attack logic
  (bind _asattack_pawn_bttask (cast `/Game/AI/Tasks/AttackPawn_BTTask` CallingTask))
  (`BTTask_BlueprintBase.FinishExecute` _asattack_pawn_bttask false))

(fn `OnRep_CurrentHP`
  (`/Game/UI/AllLevels/EnemyHealthWB.UpdateHealth` (`self.HeathBarWB`) (`KismetMathLibrary.Conv_IntToDouble` (`self.CurrentHP`))))

(fn `OnTakeDamage`
  (params (Damage :type Integer))
  (`/Engine/EditorBlueprintResources/ActorMacros.Switch Has Authority`
    (:`Authority`
      (set `self.CurrentHP` (- (`self.CurrentHP`) Damage))
      (`self.CheckDead`))))

(fn `RotateHealthBarToPlayer`
  (bind _healthbar (`self.HealthBar`))
  (bind (_returnvalue_roll _returnvalue_pitch _returnvalue_yaw) (`KismetMathLibrary.BreakRotator` (`KismetMathLibrary.FindLookAtRotation` (`SceneComponent.K2_GetComponentLocation` _healthbar) (`PlayerCameraManager.GetCameraLocation` (`GameplayStatics.GetPlayerCameraManager` 0)))))
  (`SceneComponent.K2_SetWorldRotation` _healthbar (`KismetMathLibrary.MakeRotator` _returnvalue_roll _returnvalue_pitch _returnvalue_yaw) false false))

(fn `UserConstructionScript`)