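; Tusk is a playable character with a teleporter, mana-draining flight and charge-based fireballs aimed while flying.
; Ability 1 plays a throw montage or teleports to the live teleporter and starts flight; Ability 2 toggles flight, drained by a delayed-loop macro.
; Ability 3 shows a camera-traced surface indicator until release.
; Montages route through server-to-multicast events, with separate events spawning projectiles, including a cycling special basic attack.
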(event `self.TickCooldown`
  ;[1 1 1] Tick Cooldown
  (bind _result (`/Engine/EditorBlueprintResources/StandardMacros.IncrementFloat` (`self.CurrentRegenTime`))
    (:`  `
      (if (and (>= _result (`self.MeteorRegenTime`)) (< (`self.MeteorCharges`) (`self.MaxMeteorCharges`)))
        (`/Engine/EditorBlueprintResources/StandardMacros.IncrementInt` (`self.MeteorCharges`)
          (:`  `
            (set `self.CurrentRegenTime` 0.0)))))))

(event `self.ReceiveBeginPlay`
  ;[1 1 1] Begin Play
  (bind _returnvalue (`|CreateWidget` "/Game/UI/AllLevels/Tusk_ReticleBP.Tusk_ReticleBP_C"))
  (`UserWidget.AddToViewport` _returnvalue 0)
  (`self.SetupAbilityIndicators`)
  (`KismetSystemLibrary.Delay` 0.2)
  (`self.Update Mana Widget`))

(event `self.ReceiveTick`
  (params (DeltaSeconds :type "Float (single-precision)"))
  ;[1 1 1] Event Tick
  (`self.ThirdAbilityIndicatorRaycast`)
  (`self.Debug`))

(event `SetupAbilityIndicators`
  (bind _firstabilityradius (`self.FirstAbilityRadius`))
  ;[1 1 1] Create and attach ability 1 indicator widget
  (bind _returnvalue (`|CreateWidget` "/Game/UI/AllLevels/AbilityIndicators/Tusk_1_WB.Tusk_1_WB_C"))
  (bind _returnvalue_2 (`AddComponent|NODE_AddWidgetComponent-1` :`bManualAttachment` true))
  (`WidgetComponent.SetWidget` _returnvalue_2 _returnvalue)
  (`SceneComponent.K2_AttachToComponent` _returnvalue_2 (`self.CapsuleComponent`) "None" "KeepWorld" "KeepWorld" "KeepWorld" true)
  (bind _output_get (set `self.FirstAbilityIndicator` _returnvalue_2))
  (bind _returnvalue_3 (`AddComponent|NODE_AddStaticMeshComponent-0`))
  (set `self.FirstAbilitySphere` _returnvalue_3)
  (`StaticMeshComponent.SetStaticMesh` _returnvalue_3 "/Engine/BasicShapes/Sphere.Sphere")
  (`PrimitiveComponent.SetMaterial` _returnvalue_3 0 "/Game/Textures/Tusk_1_Indicator_M.Tusk_1_Indicator_M")
  (`SceneComponent.SetVisibility` _returnvalue_3 false true)
  (`SceneComponent.SetVisibility` _returnvalue_2 false true)
  (`PrimitiveComponent.SetCollisionEnabled` _returnvalue_3 "NoCollision")
  (`SceneComponent.SetWorldScale3D` _returnvalue_3 (`KismetMathLibrary.MakeVector` _firstabilityradius _firstabilityradius _firstabilityradius))
  (`SceneComponent.K2_AttachToComponent` _returnvalue_3 _output_get "None" "KeepWorld" "KeepWorld" "KeepWorld" true))

(event `ThirdAbilityIndicatorRaycast`
  (bind _followcamera (`self.FollowCamera`))
  (bind _firstabilityindicator (`self.FirstAbilityIndicator`))
  (bind _returnvalue (`SceneComponent.K2_GetComponentLocation` _followcamera))
  ;[1 1 1] Fireball Line Trace for inidcator
  (if (`self.ThirdAbilityAimed`)
    (bind (_outhit _returnvalue_2) (`KismetSystemLibrary.LineTraceSingle` _returnvalue (+ _returnvalue (* (`SceneComponent.GetForwardVector` _followcamera) 100000.0)) "TraceTypeQuery1"))
    (if _returnvalue_2
      (bind (_bblockinghit _binitialoverlap _time _distance _location _impactpoint _normal _impactnormal _physmat _hitactor) (`GameplayStatics.BreakHitResult` _outhit))
      (`/Engine/EditorBlueprintResources/StandardMacros.IsValid` _hitactor
        (:`Is Valid`
          (if (not (or (`self.ActorHasTag` _hitactor "Enemy") (`self.ActorHasTag` _hitactor "Projectile")))
            (`SceneComponent.K2_SetWorldLocation` _firstabilityindicator (`KismetMathLibrary.MakeVector` (.x _impactpoint) (.y _impactpoint) (+ (.z _impactpoint) 10.0)) false false)
            (bind (_returnvalue_roll _returnvalue_pitch _returnvalue_yaw) (`KismetMathLibrary.BreakRotator` (`KismetMathLibrary.FindLookAtRotation` _impactpoint (* _normal 10000000.0))))
            (`SceneComponent.K2_SetWorldRotation` _firstabilityindicator (`KismetMathLibrary.MakeRotator` _returnvalue_roll _returnvalue_pitch _returnvalue_yaw) false false)
            (`SceneComponent.K2_SetWorldLocation` (`self.FirstAbilitySphere`) _impactpoint false false)))))))

(event `Multicast Spawn E Teleport FX`
  ;[1 1 1] Authority routing logic
  (`GameplayStatics.SpawnEmitterAtLocation` "/Game/Particles/Tusk_E_FX.Tusk_E_FX" (`self.K2_GetActorLocation` (`self.TeleporterRef`)) (struct) (2.0 2.0 2.0)))

(event `Server Ability 1 Logic`
  ;[1 1 1] E Ability Logic
  (`self.K2_SetActorLocation` (`self.K2_GetActorLocation` (`self.TeleporterRef`)))
  (`self.Multicast Spawn E Teleport FX`)
  (`self.Enable Flight`)
  (`self.K2_DestroyActor` (`self.TeleporterRef`)))

(event `Multicast Play E Montage`
  ;[1 1 1] Authority routing logic
  (`|PlayMontage` (`self.Mesh`) "/Game/Flight_Locomotion/Animations/RightHook_Montage.RightHook_Montage" 2.0))

(event `Debug`
  ;[1 1 1] Debug
  (`KismetSystemLibrary.PrintString` (`KismetStringLibrary.Conv_BoolToString` (`self.IsBasicAttacking`)) true true (struct :`G` 0.66 :`B` 1.0 :`A` 1.0) 0.0)
  (`KismetSystemLibrary.PrintString` (`KismetStringLibrary.Conv_IntToString` (`self.MeteorCharges`)) true true (struct :`G` 0.66 :`B` 1.0 :`A` 1.0) 0.0))

(event `InputAction|Ability 1`
  (params (Key :type "Key Structure"))
  ;[1 1 1] E Ability Logic
  (:`Pressed`
    (`/Engine/EditorBlueprintResources/StandardMacros.IsValid` (`self.TeleporterRef`)
      (:`Is Valid`
        (`self.Server Ability 1 Logic`))
      (:`Is Not Valid`
        (`self.Server Play E Montage`)))))

(event `Server Play E Montage`
  ;[1 1 1] Authority routing logic
  (`self.Multicast Play E Montage`))

(event `SpawnTeleporter`
  (bind (_returnvalue_roll _returnvalue_pitch _returnvalue_yaw) (`KismetMathLibrary.BreakRotator` (`SceneComponent.K2_GetComponentRotation` (`self.FollowCamera`))))
  ;[1 1 1] E Teleporter Spawning
  (`/Engine/EditorBlueprintResources/ActorMacros.Switch Has Authority`
    (:`Authority`
      (bind _returnvalue (`|SpawnActorFromClass` "/Game/Blueprints/Gameplay/Teleporter_BP.Teleporter_BP_C" (`KismetMathLibrary.MakeTransform` (`SceneComponent.GetSocketLocation` (`self.Mesh`) "hand_r") (`KismetMathLibrary.MakeRotator` 0.0 _returnvalue_pitch _returnvalue_yaw)) "Undefined" "OverrideRootScale" null null))
      (set `self.TeleporterRef` _returnvalue))))

(event `Multicast Play Ability 3 Montage`
  ;[1 1 1] Ability 3 Logic
  ;;[1 1 1] Authority routing logic
  (`|PlayMontage` (`self.Mesh`) "/Game/Flight_Locomotion/Animations/Air_Throw_Montage.Air_Throw_Montage" 1.5))

(event `Spawn Fireball`
  (bind (_returnvalue_roll _returnvalue_pitch _returnvalue_yaw) (`KismetMathLibrary.BreakRotator` (`SceneComponent.K2_GetComponentRotation` (`self.FollowCamera`))))
  ;[1 1 1] Spawn Fireball
  (`|SpawnActorFromClass` "/Game/Blueprints/Gameplay/Fireball_BP.Fireball_BP_C" (`KismetMathLibrary.MakeTransform` (`SceneComponent.GetSocketLocation` (`self.Mesh`) "hand_r") (`KismetMathLibrary.MakeRotator` _returnvalue_roll _returnvalue_pitch _returnvalue_yaw) (0.5 0.5 0.5)) "Undefined" "OverrideRootScale" self null)
  (set `self.MeteorCharges` (`KismetMathLibrary.Clamp` (- (`self.MeteorCharges`) 1) 0 (`self.MaxMeteorCharges`))))

(event `InputAction|Ability 3`
  (params (Key :type "Key Structure"))
  (bind _firstabilityindicator (`self.FirstAbilityIndicator`))
  (bind _returnvalue (and (`NavMovementComponent.IsFlying` (`self.CharacterMovement`)) (> (`self.MeteorCharges`) 0)))
  ;[1 1 1] Ability 3 Logic
  (:`Pressed`
    (if _returnvalue
      (set `self.ThirdAbilityAimed` true)
      (`/Engine/EditorBlueprintResources/StandardMacros.IsValid` _firstabilityindicator
        (:`Is Valid`
          (`SceneComponent.SetVisibility` _firstabilityindicator true true)))))
  (:`Released`
    (set `self.ThirdAbilityAimed` false)
    (`SceneComponent.SetVisibility` (`self.FirstAbilityIndicator`) false true)
    (if _returnvalue
      (if (not (`AnimInstance.Montage_IsPlaying` (`SkeletalMeshComponent.GetAnimInstance` (`self.Mesh`)) null))
        (`self.Server Play Ability 3 Montage`)))))

(event `Server Play Ability 3 Montage`
  ;[1 1 1] Ability 3 Logic
  ;;[1 1 1] Authority routing logic
  (`self.Multicast Play Ability 3 Montage`))

(event `Enable Flight`
  (bind _charactermovement (`self.CharacterMovement`))
  ;[1 1 1] Toggle Flight mode
  (if (> (`self.CurrentMana`) 0.0)
    (`CharacterMovementComponent.SetMovementMode` _charactermovement "MOVE_Flying" 0)
    (`self.WhileLoopWithDelay` (`NavMovementComponent.IsFlying` _charactermovement) 0.1
      (:`Body`
        (bind _output_get (set `self.CurrentMana` (- (`self.CurrentMana`) (`self.FlightManaCost`))))
        (`self.Update Mana Widget`)
        (if (<= (`KismetMathLibrary.FClamp` _output_get 0.0 (`self.ManaMax`)) 0.0)
          (`self.Disable Flight`))))))

(event `InputAction|Ability 2`
  (params (Key :type "Key Structure"))
  ;[1 1 1] Ability 2 Logic
  (:`Pressed`
    (if (`self.CanMove`)
      (if (`NavMovementComponent.IsFlying` (`self.CharacterMovement`))
        (`self.Disable Flight`)
        (else
          (`self.Enable Flight`))))))

(event `Spawn Basic Attack`
  (bind (_returnvalue_roll _returnvalue_pitch _returnvalue_yaw) (`KismetMathLibrary.BreakRotator` (`SceneComponent.K2_GetComponentRotation` (`self.FollowCamera`))))
  ;[1 1 1] Basic attack logic
  (`/Engine/EditorBlueprintResources/ActorMacros.Switch Has Authority`
    (:`Authority`
      (`|SpawnActorFromClass` (select `int` (`self.BasicAttackCounter`) :`0` "/Game/Blueprints/Gameplay/TuskBA_BP.TuskBA_BP_C" :`1` "/Game/Blueprints/Gameplay/TuskBA_BP.TuskBA_BP_C" :`2` "/Game/Blueprints/Gameplay/TuskBA_Spec_BP.TuskBA_Spec_BP_C" :!type "Actor Class Reference") (`KismetMathLibrary.MakeTransform` (`SceneComponent.GetSocketLocation` (`self.Mesh`) "hand_l") (`KismetMathLibrary.MakeRotator` _returnvalue_roll (+ _returnvalue_pitch 180.0) _returnvalue_yaw) (2.0 1.5 0.2)) "Undefined" "OverrideRootScale" self self)
      (`/Engine/EditorBlueprintResources/StandardMacros.IncrementInt` (`self.BasicAttackCounter`)
        (:`  `
          (if (>= (`self.BasicAttackCounter`) (`self.BasicAttackCounterMax`))
            (set `self.BasicAttackCounter` 0)))))))

(event `Basic Attack Pressed`
  ;[1 1 1] Basic attack logic
  (set `self.IsBasicAttacking` true)
  (if (not (`AnimInstance.Montage_IsPlaying` (`SkeletalMeshComponent.GetAnimInstance` (`self.Mesh`)) null))
    (`self.Server Play Basic Attack Montage`)
    (set `self.AttackLocked` true)))

(event `Multicast Play Basic Attack Montage`
  ;[1 1 1] Basic attack logic
  ;;[1 1 1] Authority routing logic
  (`|PlayMontage` (`self.Mesh`) "/Game/Flight_Locomotion/Animations/LeftHook_Montage.LeftHook_Montage" 2.0))

(event `InputAction|BasicAttack`
  (params (Key :type "Key Structure"))
  ;[1 1 1] Basic attack logic
  (:`Pressed`
    (`self.Basic Attack Pressed`))
  (:`Released`
    (`self.Basic Attack Released`)))

(event `Basic Attack Released`
  ;[1 1 1] Basic attack logic
  (set `self.IsBasicAttacking` false))

(event `Disable Flight`
  ;[1 1 1] Toggle Flight mode
  (`CharacterMovementComponent.SetMovementMode` (`self.CharacterMovement`) "MOVE_Walking" 0))

(event `Server Play Basic Attack Montage`
  ;[1 1 1] Basic attack logic
  ;;[1 1 1] Authority routing logic
  (`self.Multicast Play Basic Attack Montage`))

(event `InputAxis|FlyUp`
  (params (AxisValue :type "Float (single-precision)"))
  (bind (_returnvalue_x _returnvalue_y) (`KismetMathLibrary.BreakVector` (* (`KismetMathLibrary.GetForwardVector` (`self.K2_GetActorRotation`)) AxisValue)))
  ;[1 1 1] Flight Axis input
  (if (`self.CanMove`)
    (`self.AddMovementInput` (`KismetMathLibrary.MakeVector` _returnvalue_x _returnvalue_y 100.0) AxisValue)))

(event `CheckBasicAttack`
  ;[1 1 1] Check if basic attacking notify event
  (if (not (`self.IsBasicAttacking`))
    (`AnimInstance.Montage_SetNextSection` (`SkeletalMeshComponent.GetAnimInstance` (`self.Mesh`)) "Default" "End" "/Game/Flight_Locomotion/Animations/LeftHook_Montage.LeftHook_Montage")))

(event `self.LandingSphere.OnComponentBeginOverlap`
  (params (OverlappedComponent :type "PrimitiveComponent Object Reference") (OtherActor :type "Actor Object Reference") (OtherComp :type "PrimitiveComponent Object Reference") (OtherBodyIndex :type Integer) (bFromSweep :type Boolean) (SweepResult :type "HitResult Structure (by ref)"))
  ;[1 1 1] Landing Sphere hit detection
  (if (`NavMovementComponent.IsFlying` (`self.CharacterMovement`))
    (if (`self.ActorHasTag` OtherActor "Walkable")
      (`self.Disable Flight`))))

(event `Gain Mana`
  (params (Gain :type "Float (double-precision)"))
  ;[1 1 1] Gain mana logic
  (set `self.CurrentMana` (`KismetMathLibrary.FClamp` (+ Gain (`self.CurrentMana`)) 0.0 (`self.ManaMax`)))
  (`self.Update Mana Widget`))

(event `Server Check Basic Attacking`
  (`self.CheckBasicAttack`))

(event `Update Mana Widget`
  ;[1 1 1] Update Mana Widget
  (bind _asgameplay_pc (cast `/Game/Blueprints/Gameplay/GameplayPC` (`GameplayStatics.GetPlayerController` 0)))
  (`/Game/UI/AllLevels/NewPlayerHUD.UpdateResource` (`/Game/Blueprints/Gameplay/GameplayPC.HUD` _asgameplay_pc) (`self.CurrentMana`)))

(fn `GetFlightAngle`
  (returns (AngleFromYVector :type "Float (double-precision)"))
  (bind _returnvalue (`KismetMathLibrary.MakeVector2D` (`self.GetInputAxisValue`) (`self.GetInputAxisValue`)))
  (bind _returnvalue_2 (`KismetMathLibrary.DegAcos` (/ (`KismetMathLibrary.DotProduct2D` (`KismetMathLibrary.MakeVector2D` 1.0) _returnvalue) (`KismetMathLibrary.VSize2D` _returnvalue))))
  (if (== (+ (`KismetMathLibrary.Abs` (`self.GetInputAxisValue`)) (`KismetMathLibrary.Abs` (`self.GetInputAxisValue`))) 0.0)
    (return 90.0)
    (elif (< (`self.GetInputAxisValue`) 0.0)
      (return (* _returnvalue_2 (`self.GetInputAxisValue`)))
      (else
        (return _returnvalue_2)))))

(fn `UserConstructionScript`
  (`parent.UserConstructionScript`))