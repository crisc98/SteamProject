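; Frosty is a playable networked melee character that spawns twin axes into its hand sockets and fights with montage-driven combos.
; Abilities include a draining rage toggle that boosts damage, combo set and trails, plus a spin, a roll and an attack with slash projectiles.
; Input routes to server logic, with multicast montages for some abilities.
; Decrementing cooldowns and rage feed the HUD, and Tick prints debug values.
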(event `UpdateQCooldownWidget`
  (params (Value :type "Float (double-precision)"))
  ;[1 1 1] Update Q cooldown widget
  (bind _asgameplay_pc (cast `/Game/Blueprints/Gameplay/GameplayPC` (`GameplayStatics.GetPlayerController` 0)))
  (`/Game/UI/AllLevels/NewPlayerHUD.UpdateQCooldown` (`/Game/Blueprints/Gameplay/GameplayPC.HUD` _asgameplay_pc) Value))

(event `UpdateShiftCooldownWidget`
  (params (Value :type "Float (double-precision)"))
  ;[1 1 1] Update Q cooldown widget
  (bind _asgameplay_pc (cast `/Game/Blueprints/Gameplay/GameplayPC` (`GameplayStatics.GetPlayerController` 0)))
  (`/Game/UI/AllLevels/NewPlayerHUD.UpdateShiftCooldown` (`/Game/Blueprints/Gameplay/GameplayPC.HUD` _asgameplay_pc) Value))

(event `UpdateRMBCooldownWidget`
  (params (Cooldown :type "Float (double-precision)"))
  ;[1 1 1] Update Q cooldown widget
  (bind _asgameplay_pc (cast `/Game/Blueprints/Gameplay/GameplayPC` (`GameplayStatics.GetPlayerController` 0)))
  (`/Game/UI/AllLevels/NewPlayerHUD.UpdateRMBCooldown` (`/Game/Blueprints/Gameplay/GameplayPC.HUD` _asgameplay_pc) Cooldown))

(event `self.ReceiveBeginPlay`
  ;[1 1 1] Begin Play
  (`self.AttachWeapons`))

(event `self.TickCooldown`
  (`self.ResetAbility1`)
  (`self.Reset Ability 3`)
  (`self.Reset Ability 4`))

(event `ResetAbility1`
  ;[1 1 1] Setup Cooldown timer event
  (bind _output_get (set `self.QCooldown` (`KismetMathLibrary.FClamp` (- (`self.QCooldown`) 1.0) 0.0 (`self.QMaxCD`))))
  (`self.UpdateQCooldownWidget` _output_get))

(event `AttachWeapons`
  ;[1 1 1] Weapon Attach Logic
  (bind _returnvalue (`|SpawnActorFromClass` "/Game/Blueprints/Gameplay/TwinAxe_BP.TwinAxe_BP_C" (`KismetMathLibrary.MakeTransform` (0.0 5.0 30.0) (struct :`Yaw` 45.0) (0.8 0.8 0.8)) "Undefined" "OverrideRootScale" self self))
  (`SceneComponent.K2_AttachToComponent` (`Actor.RootComponent` _returnvalue) (`self.Mesh`) "hand_rSocket" "KeepRelative" "KeepRelative" "KeepRelative" true)
  (`KismetArrayLibrary.Array_Add` (`self.EquippedWeapons`) _returnvalue)
  (bind _returnvalue_2 (`|SpawnActorFromClass` "/Game/Blueprints/Gameplay/TwinAxe_BP.TwinAxe_BP_C" (`KismetMathLibrary.MakeTransform` (10.0 -5.0 0.0) (struct :`Pitch` 150.0 :`Yaw` -120.0) (0.8 0.8 0.8)) "Undefined" "OverrideRootScale" self self))
  (`SceneComponent.K2_AttachToComponent` (`Actor.RootComponent` _returnvalue_2) (`self.Mesh`) "hand_lSocket" "KeepRelative" "KeepRelative" "KeepRelative" true)
  (`KismetArrayLibrary.Array_Add` (`self.EquippedWeapons`) _returnvalue_2))

(event `Reset Ability 3`
  ;[1 1 1] Setup Cooldown timer event
  (bind _output_get (set `self.RMBCooldown` (`KismetMathLibrary.FClamp` (- (`self.RMBCooldown`) 1.0) 0.0 (`self.RMBMaxCD`))))
  (`self.UpdateRMBCooldownWidget` _output_get))

(event `Reset Ability 4`
  ;[1 1 1] Setup Cooldown timer event
  (bind _output_get (set `self.ShiftCooldown` (`KismetMathLibrary.FClamp` (- (`self.ShiftCooldown`) 1.0) 0.0 (`self.ShiftMaxCD`))))
  (`self.UpdateShiftCooldownWidget` _output_get))

(event `InputAction|BasicAttack`
  (params (Key :type "Key Structure"))
  ;[1 1 1] Basic Attack combo logic
  (:`Pressed`
    (if (`self.CanAttack`)
      (`/Engine/EditorBlueprintResources/ActorMacros.Switch Has Authority`
        (:`Authority`
          (`self.S_BasicAttack` :!label _label))
        (:`Remote`
          (`self.TellServerToBasicAttack`))))))

(event `TellServerToBasicAttack`
  ;[1 1 1] Basic Attack combo logic
  (goto _label))

(event `S_BasicAttack`
  (bind _returnvalue (`KismetMathLibrary.Min` (`self.ComboCounter`) (`self.MaxComboCounter`)))
  ;[1 1 1] Basic Attack combo logic
  (if (`NavMovementComponent.IsFalling` (`self.GetMovementComponent`))
    _
    (elif (not (`self.IsBasicAttacking`))
      (set `self.IsBasicAttacking` true)
      (`KismetArrayLibrary.Array_Clear` (`self.EnemiesHitInAttack`))
      (`self.AdjustRotatioForAttack`)
      (`self.DisableJump`)
      (bind _asanim_montage (cast `AnimMontage` (`KismetMathLibrary.SelectObject` (select `int` _returnvalue :`0` "/Game/IBWarriors/Animations/TwinSword_Attack04_Montage.TwinSword_Attack04_Montage" :`1` "/Game/IBWarriors/Animations/TwinSword_Attack05_Montage.TwinSword_Attack05_Montage" :`2` "/Game/IBWarriors/Animations/TwinSword_Attack06_Montage.TwinSword_Attack06_Montage" :`3` "/Game/IBWarriors/Animations/TwinSword_Attack07_Montage.TwinSword_Attack07_Montage" :`4` "/Game/IBWarriors/Animations/TwinSword_Attack08_Montage.TwinSword_Attack08_Montage" :`5` "/Game/IBWarriors/Animations/TwinSword_Attack09_Montage.TwinSword_Attack09_Montage" :!type "AnimMontage Object Reference") (select `int` _returnvalue :`0` "/Game/IBWarriors/Animations/TwinSword_Attack01_Montage.TwinSword_Attack01_Montage" :`1` "/Game/IBWarriors/Animations/TwinSword_Attack03_Montage.TwinSword_Attack03_Montage" :`2` "/Game/IBWarriors/Animations/TwinSword_Attack02_Montage.TwinSword_Attack02_Montage" :!type "AnimMontage Object Reference") (`self.IsInRageMode`))))
      (bind _notifyname (`|PlayMontage` (`self.Mesh`) _asanim_montage)
        (:`then`
          (`/Engine/EditorBlueprintResources/ActorMacros.Switch Has Authority`
            (:`Authority`
              (if (>= (`self.ComboCounter`) (`self.MaxComboCounter`))
                (set `self.ComboCounter` 0)
                (else
                  (set `self.ComboCounter` (+ (`self.ComboCounter`) 1)))))))
        (:`OnCompleted`
          (`/Engine/EditorBlueprintResources/ActorMacros.Switch Has Authority`
            (:`Authority`
              (set `self.ComboCounter` 0)
              (set `self.WeaponDamageEnabled` false)
              (`self.Enable Jump`))))
        (:`OnNotifyEnd`
          (`/Engine/EditorBlueprintResources/ActorMacros.Switch Has Authority`
            (:`Authority`
              (if (== _notifyname "Attack")
                (set `self.IsBasicAttacking` false)))))))))

(event `SetWeaponTrail`
  (params (Trail :type "ParticleSystem Object Reference"))
  ;[1 1 1] Set weapon trail
  (`self.S_SetWeaponTrail` Trail))

(event `S_SetWeaponTrail`
  (params (Trail :type "ParticleSystem Object Reference"))
  ;[1 1 1] Set weapon trail
  (for _array_element (`self.EquippedWeapons`)
    (bind _astwin_axe_bp (cast `/Game/Blueprints/Gameplay/TwinAxe_BP` _array_element))
    (`/Game/Blueprints/Gameplay/TwinAxe_BP.SetParticleTrail` _astwin_axe_bp Trail)))

(event `AdjustRotatioForAttack`
  (bind (_returnvalue_roll _returnvalue_pitch _returnvalue_yaw) (`KismetMathLibrary.BreakRotator` (`SceneComponent.K2_GetComponentRotation` (`self.FollowCamera`))))
  ;[1 1 1] Adjust camera for attack
  (`self.K2_SetActorRotation` (`KismetMathLibrary.MakeRotator` _returnvalue_roll 0.0 _returnvalue_yaw)))

(event `GainRage`
  (params (RageGain :type Integer))
  ;[1 1 1] Gain Rage Event
  (if (not (`self.IsInRageMode`))
    (bind _output_get (set `self.CurrentRage` (`KismetMathLibrary.Clamp` (+ RageGain (`self.CurrentRage`)) 0 (`self.RageMax`))))
    (`self.UpdateRageWidget` _output_get)))

(event `InputAction|Ability 1`
  (params (Key :type "Key Structure"))
  ;[1 1 1] Rage Ability Logic
  (:`Pressed`
    (if (not (`self.IsDead`))
      (`/Engine/EditorBlueprintResources/ActorMacros.Switch Has Authority`
        (:`Authority`
          (`self.Ability1Logic`))
        (:`Remote`
          (`self.ClientAbility1`))))))

(event `Ability1Logic`
  (bind _returnvalue (> (`self.CurrentRage`) 0))
  ;[1 1 1] Rage Ability Logic
  (if _returnvalue
    (bind _output_get (set `self.IsInRageMode` (not (`self.IsInRageMode`))))
    (if _output_get
      (set `self.MaxComboCounter` 5)
      (`self.S_SetWeaponTrail` "/Game/Particles/Rage_Sword_Trail.Rage_Sword_Trail")
      (set `self.ActiveWeaponDamage` (* (`self.ActiveWeaponDamage`) (`self.RageMultiplier`)))
      (`self.LoopWithDelay` (and _returnvalue _output_get) 0.1
        (:`LoopBody`
          (bind _result (`/Engine/EditorBlueprintResources/StandardMacros.DecrementInt` (`self.CurrentRage`))
            (:`  `
              (`self.UpdateRageWidget` _result))))
        (:`Done`
          (set `self.IsInRageMode` false)
          (`self.S_SetWeaponTrail` "/Game/Particles/Normal_Sword_Trail.Normal_Sword_Trail")
          (set `self.ActiveWeaponDamage` (/ (`self.ActiveWeaponDamage`) (`self.RageMultiplier`)))
          (set `self.MaxComboCounter` 2))))))

(event `ClientAbility1`
  ;[1 1 1] Rage Ability Logic
  (`self.Ability1Logic`))

(event `UpdateRageWidget`
  (params (InInt :type Integer))
  ;[1 1 1] Update Rage Widget
  (bind _asgameplay_pc (cast `/Game/Blueprints/Gameplay/GameplayPC` (`GameplayStatics.GetPlayerController` 0)))
  (`/Game/UI/AllLevels/NewPlayerHUD.UpdateResource` (`/Game/Blueprints/Gameplay/GameplayPC.HUD` _asgameplay_pc) (`KismetMathLibrary.Conv_IntToDouble` InInt)))

(event `InputAction|Ability 2`
  (params (Key :type "Key Structure"))
  ;[1 1 1] Spin Ability Logic
  (:`Pressed`
    (if (`self.CanAttack`)
      (`self.S_Ability2Logic`))))

(event `PlayAbility2Montage`
  ;[1 1 1] Spin Ability Logic
  (set `self.bUseControllerRotationYaw` true)
  (bind _notifyname (`|PlayMontage` (`self.Mesh`) "/Game/IBWarriors/Animations/TwinSword_Attack11_Montage.TwinSword_Attack11_Montage")
    (:`OnCompleted`
      (set `self.bUseControllerRotationYaw` false)
      (`/Engine/EditorBlueprintResources/ActorMacros.Switch Has Authority`
        (:`Authority`
          (set `self.IsBasicAttacking` false)
          (set `self.WeaponDamageEnabled` false)
          (set `self.ActiveWeaponDamage` (/ (`self.ActiveWeaponDamage`) (`self.SpinAbilityMultiplier`)) :!label _label_2)
          (`self.Enable Jump`))))
    (:`OnInterrupted`
      (goto _label_2))
    (:`OnNotifyEnd`
      (set `self.bUseControllerRotationYaw` false)
      (`/Engine/EditorBlueprintResources/ActorMacros.Switch Has Authority`
        (:`Authority`
          (if (== _notifyname "Attack")
            (set `self.IsBasicAttacking` false)))))))

(event `EnableWeaponDamage`
  ;[1 1 1] Enable Weapon Damge
  (set `self.WeaponDamageEnabled` true))

(event `self.ReceiveTick`
  (params (DeltaSeconds :type "Float (single-precision)"))
  ;[1 1 1] Debug
  (`KismetSystemLibrary.PrintString` (`KismetStringLibrary.Conv_BoolToString` (`self.IsBasicAttacking`)) true true (struct :`R` 1.0 :`A` 1.0) 0.0)
  (`KismetSystemLibrary.PrintString` (`KismetStringLibrary.Conv_IntToString` (`self.ActiveWeaponDamage`)) true true (struct :`R` 1.0 :`A` 1.0) 0.0))

(event `S_Ability2Logic`
  ;[1 1 1] Spin Ability Logic
  (if (and (== (`self.QCooldown`) 0.0) (not (`self.IsBasicAttacking`)))
    (`KismetArrayLibrary.Array_Clear` (`self.EnemiesHitInAttack`))
    (`self.AdjustRotatioForAttack`)
    (`self.DisableJump`)
    (set `self.ActiveWeaponDamage` (* (`self.ActiveWeaponDamage`) (`self.SpinAbilityMultiplier`)))
    (`self.PlayAbility2Montage`)
    (set `self.IsBasicAttacking` true)
    (set `self.QCooldown` (`self.QMaxCD`))))

(event `Multicast Ability 4`
  ;[1 1 1] Roll Ability logic
  (`|PlayMontage` (`self.Mesh`) "/Game/IBWarriors/Animations/TwinSword_Dash_Montage.TwinSword_Dash_Montage"
    (:`OnCompleted`
      _)
    (:`OnInterrupted`
      _))
  (if (not (`self.IsBasicAttacking`))
    (`self.Enable Jump`)))

(event `InputAction|Ability 4`
  (params (Key :type "Key Structure"))
  ;[1 1 1] Roll Ability logic
  (:`Pressed`
    (`self.Server Ability 4`)))

(event `Server Ability 4`
  ;[1 1 1] Roll Ability logic
  (if (and (not (`self.IsBasicAttacking`)) (== (`self.ShiftCooldown`) 0.0))
    (`self.DisableAttack`)
    (`self.DisableJump`)
    (`self.AdjustRotatioForAttack`)
    (`self.Multicast Ability 4`)
    (set `self.ShiftCooldown` (`self.ShiftMaxCD`))))

(event `ServerSetIsBasicAttacking`
  (params (IsBasicAttacking :type Boolean)))

(event `Multicast Ability 3`
  (`|PlayMontage` (`self.Mesh`) "/Game/IBWarriors/Animations/TwinSword_Attack10_Montage.TwinSword_Attack10_Montage"))

(event `InputAction|Ability 3`
  (params (Key :type "Key Structure"))
  (:`Pressed`
    (`self.Server Ability 3`)))

(event `Server Ability 3`
  (if (and (not (`self.IsBasicAttacking`)) (== (`self.RMBCooldown`) 0.0))
    (`self.DisableAttack`)
    (`self.DisableJump`)
    (`self.AdjustRotatioForAttack`)
    (set `self.WeaponDamageEnabled` true)
    (set `self.IsBasicAttacking` true)
    (`self.Multicast Ability 3`)
    (set `self.RMBCooldown` (`self.RMBMaxCD`))))

(event `RMBFinishNotify`
  (`self.Enable Jump`)
  (`self.EnableAttack`)
  (set `self.IsBasicAttacking` false))

(event `SpawnSlashProjectile`
  (bind (_returnvalue_roll _returnvalue_pitch _returnvalue_yaw) (`KismetMathLibrary.BreakRotator` (`self.K2_GetActorRotation`)))
  (bind (_returnvalue_roll_2 _returnvalue_pitch_2 _returnvalue_yaw_2) (`KismetMathLibrary.BreakRotator` (`self.K2_GetActorRotation`)))
  (bind _astwin_axe_bp (cast `/Game/Blueprints/Gameplay/TwinAxe_BP` (`|GetArrayItem` (`self.EquippedWeapons`))))
  (bind (_returnvalue_x _returnvalue_y _returnvalue_z) (`KismetMathLibrary.BreakVector` (`SceneComponent.GetSocketLocation` (`/Game/Blueprints/Gameplay/TwinAxe_BP.SkeletalMesh` _astwin_axe_bp) "Tip")))
  (`|SpawnActorFromClass` "/Game/Blueprints/Gameplay/Frosty_Slash_Bp.Frosty_Slash_BP_C" (`KismetMathLibrary.MakeTransform` (`KismetMathLibrary.MakeVector` _returnvalue_x _returnvalue_y (+ _returnvalue_z 70.0)) (`KismetMathLibrary.MakeRotator` 45.0 0.0 _returnvalue_yaw_2) (0.3 0.7 0.2)) "Undefined" "OverrideRootScale" self self)
  (bind _astwin_axe_bp_2 (cast `/Game/Blueprints/Gameplay/TwinAxe_BP` (`|GetArrayItem` (`self.EquippedWeapons`) 1)))
  (bind (_returnvalue_x_2 _returnvalue_y_2 _returnvalue_z_2) (`KismetMathLibrary.BreakVector` (`SceneComponent.GetSocketLocation` (`/Game/Blueprints/Gameplay/TwinAxe_BP.SkeletalMesh` _astwin_axe_bp_2) "Tip")))
  (`|SpawnActorFromClass` "/Game/Blueprints/Gameplay/Frosty_Slash_Bp.Frosty_Slash_BP_C" (`KismetMathLibrary.MakeTransform` (`KismetMathLibrary.MakeVector` _returnvalue_x_2 _returnvalue_y_2 (+ _returnvalue_z_2 70.0)) (`KismetMathLibrary.MakeRotator` 135.0 0.0 _returnvalue_yaw) (0.3 0.7 0.2)) "Undefined" "OverrideRootScale" self self))

(fn `UserConstructionScript`
  (`parent.UserConstructionScript`))